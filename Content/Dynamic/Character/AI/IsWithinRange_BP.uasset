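; Behavior tree decorator that checks whether the AI's controlled pawn is within range of a target actor.
; It reads the target actor and range from blackboard keys and fails when the target is invalid.
; The test compares squared distance between the two actor locations against the squared range, avoiding a square root, and passes at or inside that range.
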(fn PerformConditionCheckAI
  (params (OwnerController :type AI%20Controller%20Object%20Reference) (ControlledPawn :type Pawn%20Object%20Reference))
  (bind _targetkey (Variables|Default|GetTargetKey))
  (bind _rangekey (Variables|Default|GetRangeKey))
  (bind _returnvalue (AI|BehaviorTree|GetBlackboardValueasActor _targetkey))
  (bind _returnvalue_2 (Class|BTFunctionLibrary|GetBlackboardValueasFloat _rangekey))
  (Utilities|IsValid _returnvalue
    (:Is%20Valid
      (return (<= (Math|Vector|VectorLengthSquared (- (Transformation|GetActorLocation ControlledPawn) (Transformation|GetActorLocation _returnvalue))) (* _returnvalue_2 _returnvalue_2))))
    (:Is%20Not%20Valid
      (return false))))