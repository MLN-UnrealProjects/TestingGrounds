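; Behavior tree task that makes an AI-controlled Character_BP aim and shoot at a target.
; On execute it sets the character's aiming and shooting flags and focuses the controller on the blackboard's TargetKey actor.
; It never finishes execution itself, so it runs until aborted, when it clears both flags and the focus before finishing the abort.
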(event EventReceiveExecuteAI
  (params (OwnerController :type AI%20Controller%20Object%20Reference) (ControlledPawn :type Pawn%20Object%20Reference))
  (bind _ascharacter_bp (Utilities|Casting|CastToCharacter_BP ControlledPawn))
  (Variables|/Game/Dynamic/Character/Behaviour/Character_BP.Character_BP_C|SetbIsAiming _ascharacter_bp true)
  (Variables|/Game/Dynamic/Character/Behaviour/Character_BP.Character_BP_C|SetbIsShooting _ascharacter_bp true)
  (AI|SetFocus OwnerController (AI|BehaviorTree|GetBlackboardValueasActor (Variables|Default|GetTargetKey))))

(event EventReceiveAbortAI
  (params (OwnerController :type AI%20Controller%20Object%20Reference) (ControlledPawn :type Pawn%20Object%20Reference))
  (bind _ascharacter_bp (Utilities|Casting|CastToCharacter_BP ControlledPawn))
  (Variables|/Game/Dynamic/Character/Behaviour/Character_BP.Character_BP_C|SetbIsAiming _ascharacter_bp false)
  (Variables|/Game/Dynamic/Character/Behaviour/Character_BP.Character_BP_C|SetbIsShooting _ascharacter_bp false)
  (AI|ClearFocus OwnerController)
  (Class|BTTaskBlueprintBase|FinishAbort))