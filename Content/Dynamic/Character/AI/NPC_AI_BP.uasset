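; AI controller for guard NPCs that patrol and track sensed targets through a behavior tree.
; On BeginPlay it sets up the patrol blackboard, writes the range value and runs the guard behavior tree.
; Perception updates set or clear the blackboard target, ignoring actors tagged Enemy.
; A helper function writes an indexed waypoint from the controlled pawn's PatrolRoute component to a given blackboard key.
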(event OnTargetPerceptionUpdated(AIPerception)
  (params (Actor :type Actor%20Object%20Reference) (Stimulus :type AI%20Stimulus%20Structure))
  (CallFunction|UpdateBlackboardTargetKey (.bsuccessfullysensed Stimulus) Actor))

(event EventBeginPlay
  (bind _blackboardcomponent (Class|AIController|UseBlackboard "/Game/Dynamic/Character/AI/PatrolData.PatrolData"))
  (bind _output_get (Variables|Default|SetBlackboardComponent _blackboardcomponent))
  (AI|Components|Blackboard|SetValueasFloat _output_get (Variables|Default|GetBlackboardRangeKeyName) (Variables|Default|GetRange))
  (AI|RunBehaviorTree "/Game/Dynamic/Character/AI/GuardBehaviour_BP.GuardBehaviour_BP"))

(fn ConstructionScript)

(fn SelectWaypointRoute
  (params (Blackboard :type Blackboard%20Component%20Object%20Reference) (BlackboardParamName :type Name) (Index :type Integer))
  (AI|Components|Blackboard|SetValueasObject Blackboard BlackboardParamName (Utilities|Array|Get(acopy) (Class|PatrolRoute|GetPatrolLocations (Actor|GetComponentbyClass (Pawn|GetControlledPawn) "/Script/TestingGrounds.PatrolRoute")) Index)))

(fn UpdateBlackboardTargetKey
  (params (IsOtherActorSensed :type Boolean) (OtherActor :type Actor%20Object%20Reference))
  (bind _blackboardcomponent (Variables|Default|GetBlackboardComponent))
  (bind _blackboardtargetkeyname (Variables|Default|GetBlackboardTargetKeyName))
  (if (not (Actor|ActorHasTag OtherActor "Enemy"))
    (if IsOtherActorSensed
      (AI|Components|Blackboard|SetValueasObject _blackboardcomponent _blackboardtargetkeyname OtherActor)
      (else
        (AI|Components|Blackboard|ClearValue _blackboardcomponent _blackboardtargetkeyname)))))