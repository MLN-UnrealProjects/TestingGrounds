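; AI controller for NPCs that patrol and fire on sensed targets.
; It initializes the PatrolData blackboard and runs the Patrol_BP behavior tree; perception sets or clears the blackboard target for actors without the Enemy tag.
; Tick switches the controlled character's aiming and shooting on whenever a focus actor exists.
; SelectWaypointRoute writes an indexed entry from the pawn's PatrolRoute component into a given blackboard key.
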(event OnTargetPerceptionUpdated(AIPerception)
  (params (Actor :type Actor%20Object%20Reference) (Stimulus :type AI%20Stimulus%20Structure))
  (bind _blackboardcomponent (Variables|Default|GetBlackboardComponent))
  (bind _blackboardtargetkeyname (Variables|Default|GetBlackboardTargetKeyName))
  (if (not (Actor|ActorHasTag Actor "Enemy"))
    (if (.bsuccessfullysensed Stimulus)
      (AI|Components|Blackboard|SetValueasObject _blackboardcomponent _blackboardtargetkeyname Actor)
      (else
        (AI|Components|Blackboard|ClearValue _blackboardcomponent _blackboardtargetkeyname)))))

(event EventBeginPlay
  (bind _blackboardcomponent (Class|AIController|UseBlackboard "/Game/Dynamic/NPC/AI/PatrolData.PatrolData"))
  (Variables|Default|SetBlackboardComponent _blackboardcomponent)
  (AI|RunBehaviorTree "/Game/Dynamic/NPC/AI/Patrol_BP.Patrol_BP"))

(event EventTick
  (params (DeltaSeconds :type Float%20%28single-precision%29))
  (bind _returnvalue (Class|AIController|GetFocusActor))
  (bind _returnvalue_2 (Utilities|IsValid _returnvalue))
  (bind _asue_4asp_character (Utilities|Casting|CastToUe4ASP_Character (Pawn|GetControlledPawn)))
  (Variables|/Game/Dynamic/NPC/Behaviour/Ue4ASP_Character.Ue4ASP_Character_C|SetbIsAiming _asue_4asp_character _returnvalue_2)
  (Variables|/Game/Dynamic/NPC/Behaviour/Ue4ASP_Character.Ue4ASP_Character_C|SetbIsShooting _asue_4asp_character _returnvalue_2))

(fn ConstructionScript)

(fn SelectWaypointRoute
  (params (Blackboard :type Blackboard%20Component%20Object%20Reference) (BlackboardParamName :type Name) (Index :type Integer))
  (AI|Components|Blackboard|SetValueasObject Blackboard BlackboardParamName (Utilities|Array|Get(acopy) (Class|PatrolRoute|GetPatrolLocations (Actor|GetComponentbyClass (Pawn|GetControlledPawn) "/Script/TestingGrounds.PatrolRoute")) Index)))