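; Terrain tile for an infinite terrain system, with an attach point for chaining and a front barrier that gates passage.
; Entering the locking volume turns the barrier green and passable.
; Leaving it turns the barrier red and solid, has the game mode spawn another tile, and flags this one for removal.
; Once flagged, the tile destroys itself when an overlap with its destroy volume ends.
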(event OnComponentBeginOverlap(LockingVolume)
  (params (OverlappedComponent :type Primitive%20Component%20Object%20Reference) (OtherActor :type Actor%20Object%20Reference) (OtherComp :type Primitive%20Component%20Object%20Reference) (OtherBodyIndex :type Integer) (bFromSweep :type Boolean) (SweepResult :type Hit%20Result%20Structure%20%28by%20ref%29))
  (if (not (Variables|Default|GetbIsReadyForDestroy))
    (Utilities|IsPlayerActor OtherActor)
    (CallFunction|UnlockBarrier)))

(event OnComponentEndOverlap(LockingVolume)
  (params (OverlappedComponent :type Primitive%20Component%20Object%20Reference) (OtherActor :type Actor%20Object%20Reference) (OtherComp :type Primitive%20Component%20Object%20Reference) (OtherBodyIndex :type Integer))
  (if (not (Variables|Default|GetbIsReadyForDestroy))
    (Utilities|IsPlayerActor OtherActor)
    (CallFunction|LockBarrier)
    (bind _asinfinite_terrain_gamemode_bp (Utilities|Casting|CastToInfiniteTerrainGamemode_BP (Game|GetGameMode)))
    (Default|SpawnTiles _asinfinite_terrain_gamemode_bp 1)
    (Variables|Default|SetbIsReadyForDestroy true)))

(event OnComponentEndOverlap(DestroyVolume)
  (params (OverlappedComponent :type Primitive%20Component%20Object%20Reference) (OtherActor :type Actor%20Object%20Reference) (OtherComp :type Primitive%20Component%20Object%20Reference) (OtherBodyIndex :type Integer))
  (if (Variables|Default|GetbIsReadyForDestroy)
    (Utilities|IsPlayerActor OtherActor)
    (Actor|DestroyActor)))

(fn ConstructionScript)

(fn GetAttachTransform
  (return (Transformation|GetWorldTransform (Variables|Default|GetArrow))))

(fn UnlockBarrier
  (bind _frontbarrier (Variables|Default|GetFrontBarrier))
  (Collision|SetCollisionEnabled _frontbarrier "NoCollision")
  (Rendering|Material|SetMaterial _frontbarrier 0 "/Game/Static/Terrain/GreenBarrier_M.GreenBarrier_M"))

(fn LockBarrier
  (bind _frontbarrier (Variables|Default|GetFrontBarrier))
  (Collision|SetCollisionEnabled _frontbarrier "QueryAndPhysics")
  (Rendering|Material|SetMaterial _frontbarrier 0 "/Game/Static/Terrain/RedBarrier_M.RedBarrier_M"))