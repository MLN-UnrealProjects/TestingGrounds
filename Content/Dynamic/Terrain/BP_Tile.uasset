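; Terrain tile for an infinite terrain game that randomly scatters props, rocks and AI characters on BeginPlay.
; An Arrow component supplies the attach transform for tile placement.
; The player entering LockingVolume opens the green front barrier; leaving turns it solid red and arms destruction.
; When the player then exits DestroyVolume, the tile destroys itself and asks GM_InfiniteTerrain to spawn a new one.
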(event OnComponentBeginOverlap(LockingVolume)
  (params (OverlappedComponent :type Primitive%20Component%20Object%20Reference) (OtherActor :type Actor%20Object%20Reference) (OtherComp :type Primitive%20Component%20Object%20Reference) (OtherBodyIndex :type Integer) (bFromSweep :type Boolean) (SweepResult :type Hit%20Result%20Structure%20%28by%20ref%29))
  (Utilities|IsPlayerActor OtherActor)
  (CallFunction|UnlockBarrier)
  (Variables|Default|SetbReadyForDestroy false))

(event OnComponentEndOverlap(LockingVolume)
  (params (OverlappedComponent :type Primitive%20Component%20Object%20Reference) (OtherActor :type Actor%20Object%20Reference) (OtherComp :type Primitive%20Component%20Object%20Reference) (OtherBodyIndex :type Integer))
  (Utilities|IsPlayerActor OtherActor)
  (CallFunction|LockBarrier)
  (Variables|Default|SetbReadyForDestroy true))

(event OnComponentEndOverlap(DestroyVolume)
  (params (OverlappedComponent :type Primitive%20Component%20Object%20Reference) (OtherActor :type Actor%20Object%20Reference) (OtherComp :type Primitive%20Component%20Object%20Reference) (OtherBodyIndex :type Integer))
  (if (Variables|Default|GetbReadyForDestroy)
    (Utilities|IsPlayerActor OtherActor)
    (bind _asgm_infinite_terrain (Utilities|Casting|CastToGM_InfiniteTerrain (Game|GetGameMode)))
    (Actor|DestroyActor)
    (Default|SpawnTiles _asgm_infinite_terrain 1)))

(event EventBeginPlay
  (Class|Tile|PlaceActors "/Game/Dynamic/Terrain/Props/BP_Box.BP_Box_C" (Utilities|Struct|MakeHOTRELOADED_TileSpawnParameters_0 7 1 1e+02 150 1.0 1.0))
  (Class|Tile|PlaceActors "/Game/Dynamic/Terrain/Props/BP_Canister.BP_Canister_C" (Utilities|Struct|MakeHOTRELOADED_TileSpawnParameters_0 10 1 5e+01 200 1.0 1.0))
  (Class|Tile|PlaceActors "/Game/Dynamic/Terrain/Props/BP_Container.BP_Container_C" (Utilities|Struct|MakeHOTRELOADED_TileSpawnParameters_0 4 1 4.3e+02 50 0.9 1.1))
  (Class|Tile|PlaceActors "/Game/Dynamic/Terrain/Props/BP_Rock_01.BP_Rock_01_C" (Utilities|Struct|MakeHOTRELOADED_TileSpawnParameters_0 5 1 2.4e+02 50 0.1 5.0))
  (Class|Tile|PlaceActors "/Game/Dynamic/Terrain/Props/BP_Rock_02.BP_Rock_02_C" (Utilities|Struct|MakeHOTRELOADED_TileSpawnParameters_0 5 1 1.5e+02 50 0.1 5.0))
  (Class|Tile|PlaceActors "/Game/Dynamic/Terrain/Props/BP_Rock_03.BP_Rock_03_C" (Utilities|Struct|MakeHOTRELOADED_TileSpawnParameters_0 5 1 2.1e+02 50 0.1 5.0))
  (Class|Tile|PlaceActors "/Game/Dynamic/Terrain/Props/BP_Sandbags.BP_Sandbags_C" (Utilities|Struct|MakeHOTRELOADED_TileSpawnParameters_0 5 1 2.1e+02 50 0.8 1.2))
  (Class|Tile|PlaceAIPawns "/Game/Dynamic/Character/Behaviour/BP_Character.BP_Character_C" (Utilities|Struct|MakeHOTRELOADED_TileAIPawnSpawnParameters_1 10 2 5e+01 200 "Enemy"))
  (Variables|Default|SetbReadyForDestroy false))

(fn ConstructionScript)

(fn GetAttachTransform
  (return (Transformation|GetWorldTransform (Variables|Default|GetArrow))))

(fn UnlockBarrier
  (bind _frontbarrier (Variables|Default|GetFrontBarrier))
  (Collision|SetCollisionEnabled _frontbarrier "NoCollision")
  (Rendering|Material|SetMaterial _frontbarrier 0 "/Game/Static/Terrain/MI_Barrier_Green.MI_Barrier_Green"))

(fn LockBarrier
  (bind _frontbarrier (Variables|Default|GetFrontBarrier))
  (Collision|SetCollisionEnabled _frontbarrier "QueryAndPhysics")
  (Rendering|Material|SetMaterial _frontbarrier 0 "/Game/Static/Terrain/MI_Barrier_Red.MI_Barrier_Red"))