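; Game mode for an infinite terrain level that lays out a chain of BP_Tile actors.
; On BeginPlay it calls PopulateBoundsInPool, defined outside this graph, then spawns an initial run of tiles.
; SpawnTiles hands each tile the shared NavMeshBoundsPool and takes its attach transform as the next spawn position, so tiles connect end to end.
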(event EventBeginPlay
  (Class|InfiniteTerrainGameMode|PopulateBoundsinPool)
  (CallFunction|SpawnTiles 4))

(fn ConstructionScript)

(fn SpawnTiles
  (params (NumberOfTilesToSpawn :type Integer))
  (if (> NumberOfTilesToSpawn 0)
    (for _index (range 1 NumberOfTilesToSpawn)
      (bind _returnvalue (Game|SpawnActorfromClass "/Game/Dynamic/Terrain/BP_Tile.BP_Tile_C" (Variables|Default|GetSpawnPosition) "AlwaysSpawn" 0 0))
      (Class|Tile|SetNavMeshBoundsPool _returnvalue (Variables|Default|GetNavMeshBoundsPool))
      (Variables|Default|SetSpawnPosition (Default|GetAttachTransform _returnvalue)))))